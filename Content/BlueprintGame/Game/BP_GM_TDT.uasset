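; Game mode that spawns players on login and turns them into death spectators when killed.
; PostLogin queues controllers, gathers BP_PlayerSpawn points there because it can precede BeginPlay, then spawns and possesses a first-person character at a random point.
; A retry macro polls for the controlled pawn before dequeuing the player.
; Each character's Killed event is bound to replace it with an initialized BP_Spectator_Death, keeping location and yaw.
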(event `Event | Player Killed`
  (params (Controller :type "Controller Object Reference") (Killer :type "Actor Object Reference"))
  ;[0 0 0] Event | Player Killed
  (`self.SpawnSpectator` Controller Killer))

(event `self.K2_PostLogin`
  (params (NewPlayer :type "PlayerController Object Reference"))
  (bind _players_awaitinglogin (`self.Players_AwaitingLogin`))
  ;[0 0 0] Event Post Login
  ;;[0.02431 0.02431 0.02431] Add to waiting players
  (if (not (`KismetArrayLibrary.Array_Contains` _players_awaitinglogin NewPlayer))
    (`KismetArrayLibrary.Array_Add` _players_awaitinglogin NewPlayer) ; I use an array in this instance to make sure\nthat players are truely spawned. If they don't\nsucceed with the following logic, they will still\nbe in this array as a reference.
  )
  ;;[0.3455 0.3455 0.3455 1 12] Normally the creation of this value would be on begin play, but due to player spawning before GM getting Begin Play, I put it here. There are many work-arounds to this.
  ;;
  ;; Honestly, if I were building a full system for login (which i've done) I would have the Player State **request** login through the Player controller. The Player State spawns after Game State, Game State spawns after Game Mode, fixing the problem. I would route it through the Player Controller because Player Controller has owning connection, which is required to access the GM (for events/functions/anything else). It also gives you the ability to accept/deny an incoming login request for any reason.
  (bind _outactors (`GameplayStatics.GetAllActorsOfClass` "/Game/BlueprintGame/Player/BP_PlayerSpawn.BP_PlayerSpawn_C"))
  (set `self.PlayerSpawns` _outactors)
  ;;[0.02431 0.02431 0.02431] Loop through waiting players and Spawn
  (for (_array_element _array_index) (`self.Players_AwaitingLogin`)
    (`self.SpawnPlayer` _array_element)
    (`self.WaitForControlledPawn` _array_element 0.25 12 ; Wait up to 3 seconds for pawn
      (:`Valid`
        (`KismetArrayLibrary.Array_Remove` (`self.Players_AwaitingLogin`) _array_index) ; Remove from Awaiting Players
      ))))

(fn `GetRandomPlayerSpawnTransform`
  (returns (Transform :type "Transform Structure"))
  (bind _playerspawns (`self.PlayerSpawns`))
  (return (`self.GetTransform` (`|GetArrayItem` _playerspawns (`KismetMathLibrary.RandomInteger` (`KismetArrayLibrary.Array_LastIndex` _playerspawns))))))

(fn `SpawnPlayer`
  (params (Controller :type "Controller Object Reference"))
  ;[0.02431 0.02431 0.02431] Create and Possess Pawn
  (bind _returnvalue (`|SpawnActorFromClass` "/Game/BlueprintGame/Player/BP_FirstPersonCharacter.BP_FirstPersonCharacter_C" (`self.GetRandomPlayerSpawnTransform`) "Undefined" "OverrideRootScale" Controller null))
  (`Controller.Possess` Controller _returnvalue)
  ;[0.02431 0.02431 0.02431] Bind "Player Killed" Event
  (add `/Game/BlueprintGame/Player/BP_FirstPersonCharacter.Killed` _returnvalue (`|CreateDelegate` :!event `Event | Player Killed`)))

(fn `SpawnSpectator`
  (params (Controller :type "Controller Object Reference") (Killer :type "Actor Object Reference"))
  (locals (LocalController :type "Controller Object Reference"))
  ;[0.07986 0.07986 0.07986] Init Local Data
  (bind _output_get (set `local.LocalController` Controller))
  (bind _returnvalue (`self.GetTransform` _output_get))
  ;[0.07986 0.07986 0.07986] Create Pawn
  (bind _returnvalue_2 (`|SpawnActorFromClass` "/Game/BlueprintGame/Player/BP_Spectator_Death.BP_Spectator_Death_C" (`KismetMathLibrary.MakeTransform` (.location _returnvalue) (`KismetMathLibrary.MakeRotator` 0.0 0.0 (.yaw (.rotation _returnvalue))) (.scale _returnvalue)) "Undefined" "OverrideRootScale" (`local.LocalController`) 0.35 1.0 0.35 null))
  ;[0.07986 0.07986 0.07986] Destroy Old Pawn if New Pawn Valid
  (`/Engine/EditorBlueprintResources/StandardMacros.IsValid` _returnvalue_2
    (:`Is Valid`
      (`self.K2_DestroyActor` (`Controller.K2_GetPawn` (`local.LocalController`)))
      ;[0.07986 0.07986 0.07986] Possess
      (`Controller.Possess` (`local.LocalController`) _returnvalue_2)
      ;[0.07986 0.07986 0.07986] Initialize Spectator
      (`/Game/BlueprintGame/Player/BP_Spectator_Death.Event | Initialize Spectator` _returnvalue_2))))

(fn `UserConstructionScript`)