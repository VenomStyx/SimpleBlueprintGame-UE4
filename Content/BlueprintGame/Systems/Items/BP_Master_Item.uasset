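; Base pickup item that spins in the world and adds itself to the inventory of a Character that touches it.
; On BeginPlay it loads its item data by ItemID from a data table, warning if missing, and starts a looping yaw timeline.
; Overlapping the radius-configurable pickup sphere either collects it immediately or, with magnet enabled, disables collision and lerps it toward the Character first.
; Collection requests an inventory add, then destroys the actor.
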(event `self.ReceiveBeginPlay`
  ;[0 0 0] Event | Begin Play
  (`self.LoadItemSettings`) ; Loads settings from data table
  (`self.Initialize Item Rotation`) ; Starts Item Rotation
)

(event `Initialize Item Pickup`
  (params (Actor :type "Actor Object Reference"))
  ;[0 0 0] Event | Initialize Item Pickup
  (if (`self.UsesItemMagnet`)
    (`self.Magnet To Actor` Actor)
    (else
      (`self.Item Picked Up` Actor))))

(event `self.PickupSphere.OnComponentBeginOverlap`
  (params (OverlappedComponent :type "PrimitiveComponent Object Reference") (OtherActor :type "Actor Object Reference") (OtherComp :type "PrimitiveComponent Object Reference") (OtherBodyIndex :type Integer) (bFromSweep :type Boolean) (SweepResult :type "HitResult Structure (by ref)"))
  ;[0 0 0] Begin Overlap | Pickup Sphere
  ;;[0.02431 0.02431 0.02431] Add Item to Inventory if Character
  (bind _ascharacter (cast `Character` OtherActor)) ; Make sure it's a player
  (`self.Initialize Item Pickup` _ascharacter))

(event `Magnet To Actor`
  (params (Actor :type "Actor Object Reference"))
  (bind (_returnvalue_x _returnvalue_y) (`KismetMathLibrary.BreakVector` (`self.K2_GetActorLocation` Actor)))
  ;[0 0 0] Event | Magnet To Actor
  ;;[0.02431 0.02431 0.02431] Update Collision Settings
  (`PrimitiveComponent.SetCollisionEnabled` (`self.PickupSphere`) "NoCollision")
  ;;[0.02431 0.02431 0.02431] Magnet Timeline
  (bind (_direction _progress) (`Timeline|Timeline_0` :!via `PlayFromStart`)
    (:`Update`
      (`self.K2_SetActorLocation` (`KismetMathLibrary.VLerp` (`self.K2_GetActorLocation`) (`KismetMathLibrary.MakeVector` _returnvalue_x _returnvalue_y) _progress)))
    (:`Finished`
      (`self.Item Picked Up` Actor))))

(event `Item Picked Up`
  (params (Actor :type "Actor Object Reference"))
  ;[0 0 0] Event | Item Picked Up
  ;;[0.02431 0.02431 0.02431] Add to Actor Inventory
  (`/Game/BlueprintGame/Systems/Items/BP_Inventory_C.Request | Add Item To Inventory` (`/Game/BlueprintGame/Game/Utilities/TDT_FL.GetInventoryFromActor` Actor) (`self.LocalItem`))
  ;;[0.02431 0.02431 0.02431] Delay & Destroy
  (`self.K2_DestroyActor`))

(event `Initialize Item Rotation`
  ;[0 0 0] Event | Initialize Item Rotation
  ;;[0.02431 0.02431 0.02431] Timeline | Item Rotation Loop
  (bind (_direction _360_float) (`Timeline|Timeline | Item Rotation` :!label _label)
    (:`Update`
      (`SceneComponent.K2_SetWorldRotation` (`self.DefaultSceneRoot`) (`KismetMathLibrary.MakeRotator` 0.0 0.0 _360_float) false false))
    (:`Finished`
      (goto _label :!via `PlayFromStart`))))

(fn `LoadItemSettings`
  (bind _itemid (`self.ItemID`))
  (bind (_valid _item_data) (`/Game/BlueprintGame/Game/Utilities/TDT_FL.GetItemDataByID` _itemid))
  ;[0.07986 0.07986 0.07986] Load Settings from Data Table by defined Item ID
  (if _valid
    (set `self.LocalItem` _item_data)
    (else
      (`KismetSystemLibrary.PrintString` (`KismetStringLibrary.Concat_StrStr` "|||WARNING||| \nITEM " (`KismetStringLibrary.Conv_IntToString` _itemid) " NOT FOUND \nPLEASE CHECK ITEM ID WITH ITEM DATATABLE")))))

(fn `UserConstructionScript`
  ;[0.07986 0.07986 0.07986] Update Pickup Sphere Radius
  (`SphereComponent.SetSphereRadius` (`self.PickupSphere`) (`self.PickupRadius`) true)
  (`SphereComponent.SetSphereRadius` (`self.PickupSphere`) (`self.PickupRadius`) true))