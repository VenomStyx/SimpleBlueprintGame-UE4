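; Interaction component for a pawn that lets the player trigger interactable actors they look at.
; On BeginPlay it waits for a valid owner, then caches the pawn's first camera through an overridable getter.
; Interact input line-traces forward from that camera on Visibility, seeking a BP_Interactable component on the hit actor.
; EventInteract fires both inside the trace function and again in the input handler, so each successful press calls it twice.
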(event `self.ReceiveBeginPlay`
  (bind (_valid _camera) (`self.GetOwningPlayerCamera` 0))
  ;[0 0 0] Event | Begin Play
  ;;[0.02431 0.02431 0.02431] Wait for & Set Camera Reference
  (`/Game/BlueprintGame/Game/Utilities/TDT_ML_ActorComponent.WaitForValidity` (`self.GetOwner`) 0.25 30
    (:`IsValid`
      (if _valid
        (set `self.PlayerCameraRef` _camera)))))

(event `Input | Interact`
  ;[0 0 0] Input | Interact
  (bind (_valid _return) (`self.TraceForInteractable`))
  (if _valid
    (`/Game/BlueprintGame/Systems/Interactables/BP_Interactable_C.Event | Interact` _return (`self.GetOwner`))))

(fn `GetOwningPawn`
  (returns (Pawn :type "Pawn Object Reference") (Valid :type Boolean))
  (bind _aspawn (cast `Pawn` (`self.GetOwner`))
    (:`then`
      (return _aspawn true))
    (:`CastFailed`
      (return null false))))

(fn `GetOwningPlayerCamera`
  (params (CameraIndex :type Integer))
  (returns (Valid :type Boolean) (Camera :type "CameraComponent Object Reference"))
  (bind (_pawn _valid) (`self.GetOwningPawn`))
  (bind _output (`|GetArrayItem` (`Actor.K2_GetComponentsByClass` _pawn "/Script/Engine.CameraComponent") CameraIndex))
  ;[0.07986 0.07986 0.07986] Get player camera at index. Can be overriden to change trace logic
  (if _valid
    (`/Engine/EditorBlueprintResources/StandardMacros.IsValid` _output
      (:`Is Valid`
        (return true _output))
      (:`Is Not Valid`
        _)))
  (return false null))

(fn `TraceForInteractable`
  (returns (Valid :type Boolean) (Return :type "/Game/BlueprintGame/Systems/Interactables/BP_Interactable_C Object Reference"))
  (bind (_start _end _valid) (`/Game/BlueprintGame/Game/Utilities/TDT_FL.GetForwardTraceLocations_SceneComponent` (`self.PlayerCameraRef`) (`self.Interaction Distance`)))
  ;[0.07986 0.07986 0.07986] Trace & Interact
  (if _valid
    (bind (_outhit _returnvalue) (`KismetSystemLibrary.LineTraceSingle` _start _end "TraceTypeQuery1")) ; Line Trace from Camera
    (if _returnvalue
      (bind _returnvalue_2 (`Actor.GetComponentByClass` (`.HitActor` (`GameplayStatics.BreakHitResult` _outhit)) "/Game/BlueprintGame/Systems/Interactables/BP_Interactable_C.BP_Interactable_C_C"))
      (`/Engine/EditorBlueprintResources/StandardMacros.IsValid` _returnvalue_2 ; Check for Valid Interactable\nComponent on Hit Actor
        (:`Is Valid`
          (`/Game/BlueprintGame/Systems/Interactables/BP_Interactable_C.Event | Interact` _returnvalue_2 (`self.GetOwner`)) ; Interact if Found
          ;[0.07986 0.07986 0.07986] Return
          (return true _returnvalue_2))
        (:`Is Not Valid`
          _))))
  (return false null))