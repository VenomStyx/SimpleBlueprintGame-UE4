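; Highway obstacle that loops a car from its start position to a GOAL point and damages any Character it hits.
; A timeline lerps the car body, and each finished run re-randomizes speed, color and restart delay before replaying.
; Color is applied through dynamic material instances created for body and roof at BeginPlay.
; On a hit, the car deals heavy damage, pauses for a delay, then resumes its run.
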(event `self.Car_BoxCollision.OnComponentBeginOverlap`
  (params (OverlappedComponent :type "PrimitiveComponent Object Reference") (OtherActor :type "Actor Object Reference") (OtherComp :type "PrimitiveComponent Object Reference") (OtherBodyIndex :type Integer) (bFromSweep :type Boolean) (SweepResult :type "HitResult Structure (by ref)"))
  ;[0 0 0] Begin Overlap | Initiate Car Hitting Player
  (bind _ascharacter (cast `Character` OtherActor))
  (`self.Event | Initiate Car Hitting Player` _ascharacter))

(event `self.ReceiveBeginPlay`
  ;[0 0 0] Event | Begin Play
  ;;[0.02431 0.02431 0.02431] Init Car Data
  (`self.Initialize Car Data`)
  (`self.Event | Generate and Play Car`) ; Generate Car & Play Timeline
)

(event `Event | Initiate Car Hitting Player`
  (params (`Hit Player` :type "Actor Object Reference"))
  ;[0 0 0] Event | Initiate Car Hitting Player
  (`GameplayStatics.ApplyDamage` `Hit Player` 150.0 null self)
  (`TimelineComponent.Stop` (`self.CarMovementTimeline`))
  (`KismetSystemLibrary.Delay` (`self.PostPlayerKilledMovementDelay`))
  (`self.Event | Play Car Movement`))

(event `Event | Play Car Movement`
  ;[0 0 0] Car Generation & Movement
  ;;[0.02431 0.02431 0.02431] Timeline | Car Movement
  (bind (_direction _progress) (`Timeline|CarMovementTimeline` :!label _label)
    (:`Update`
      (`SceneComponent.K2_SetWorldLocation` (`self.Car_Body`) (`KismetMathLibrary.VLerp` (`self.StartingLocation`) (`self.GoalLocation`) _progress) false false))
    (:`Finished`
      ;;[0.02431 0.02431 0.02431] Loop
      (`self.Event | Generate and Play Car`))))

(event `Event | Generate and Play Car`
  ;[0 0 0] Car Generation & Movement
  ;;[0.02431 0.02431 0.02431] Randomize Car data (Speed, Color, Delay between cars)
  (`self.Randomize Car Settings`)
  ;;[0.02431 0.02431 0.02431] Delay based on Settings
  (`KismetSystemLibrary.Delay` (`self.CarRestartDelay`))
  (goto _label :!via `PlayFromStart`))

(fn `Initialize Car Data`
  ;[0.07986 0.07986 0.07986] Set Initial Locations
  (set `self.StartingLocation` (`SceneComponent.K2_GetComponentLocation` (`self.Car_Body`)))
  (set `self.GoalLocation` (`SceneComponent.K2_GetComponentLocation` (`self.GOAL`)))
  ;[0.07986 0.07986 0.07986] Create & Add References for Car Body Material Instances
  (bind _returnvalue (`PrimitiveComponent.CreateDynamicMaterialInstance` (`self.Car_Body`) 0 "/Game/BlueprintGame/WorldEnemies/MATs/MAT_CarBody.MAT_CarBody" "None"))
  (`KismetArrayLibrary.Array_Add` (`self.CarMaterialInstances`) _returnvalue)
  (bind _returnvalue_2 (`PrimitiveComponent.CreateDynamicMaterialInstance` (`self.Car_Roof`) 0 "/Game/BlueprintGame/WorldEnemies/MATs/MAT_CarBody.MAT_CarBody" "None"))
  (`KismetArrayLibrary.Array_Add` (`self.CarMaterialInstances`) _returnvalue_2))

(fn `Randomize Car Settings`
  (locals (LocalR :type "Float (double-precision)" :default 0.0) (LocalB :type "Float (double-precision)" :default 0.0) (LocalG :type "Float (double-precision)" :default 0.0))
  (bind _returnvalue (`KismetMathLibrary.RandomFloatInRange` 0.0 1.0))
  ;[0.07986 0.07986 0.07986] Car Speed
  (`TimelineComponent.SetPlayRate` (`self.CarMovementTimeline`) (`KismetMathLibrary.RandomFloatInRange` (`self.CarMinSpeed`) (`self.CarMaxSpeed`)))
  ;[0.07986 0.07986 0.07986] Color
  (set `local.LocalR` _returnvalue)
  (set `local.LocalG` _returnvalue)
  (set `local.LocalG` _returnvalue)
  (for _array_element (`self.CarMaterialInstances`)
    (`MaterialInstanceDynamic.SetVectorParameterValue` _array_element "CarColor" (`KismetMathLibrary.MakeColor` (`local.LocalR`) (`local.LocalB`) (`local.LocalG`))))
  ;[0.07986 0.07986 0.07986] Car "Spawn" Delay
  (set `self.CarRestartDelay` (`KismetMathLibrary.RandomFloatInRange` (`self.MinCarRestartDelay`) (`self.MaxCarRestartDelay`))))

(fn `UserConstructionScript`)