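; Laser hazard that switches on and off at random intervals and damages characters inside its beam.
; From BeginPlay, a loop waits a random delay, enables the cylinder's visibility and collision for a set time, then disables both until ShouldStopLaser is set.
; A character overlap starts one shared looping timer, which immediately and then periodically applies damage to every overlapping character.
; The timer is cleared when the last character leaves.
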(event `self.ReceiveBeginPlay`
  ;[0 0 0] Event | Begin Play
  (`self.DisableLaser`)
  (`self.Event | Begin Laser Loop`))

(event `self.LaserCylinder.OnComponentBeginOverlap`
  (params (OverlappedComponent :type "PrimitiveComponent Object Reference") (OtherActor :type "Actor Object Reference") (OtherComp :type "PrimitiveComponent Object Reference") (OtherBodyIndex :type Integer) (bFromSweep :type Boolean) (SweepResult :type "HitResult Structure (by ref)"))
  ;[0 0 0] Event | Component Begin Overlap
  ;;[0.02431 0.02431 0.02431] Is it a character?
  (cast `Character` OtherActor)
  ;;[0.02431 0.02431 0.02431] If damage timer isn't already started, begin damage timer
  (if (not (`KismetSystemLibrary.K2_IsValidTimerHandle` (`self.DamageLoopTimerHandle`)))
    (`self.Timer | Start Damage Loop`)))

(event `Event | Begin Laser Loop`
  ;[0 0 0] Event | Begin Laser Loop
  ;;[0.02431 0.02431 0.02431] Laser Loop
  (if (not (`self.ShouldStopLaser`)) :!label _label
    (`KismetSystemLibrary.Delay` (`KismetMathLibrary.RandomFloatInRange` (`self.LaserDelay_Min`) (`self.LaserDelay_Max`)))
    (`self.EnableLaser`)
    (`KismetSystemLibrary.Delay` (`self.LazerOnTime`))
    (`self.DisableLaser`)
    (goto _label)))

(event `Timer | Start Damage Loop`
  ;[0 0 0] Damage Overlapping Players
  ;;[0.02431 0.02431 0.02431] Start Damage Timer
  (`self.Timer | Damage Loop`)
  (bind _returnvalue (`KismetSystemLibrary.K2_SetTimerDelegate` (delegate `Timer | Damage Loop`) (`self.Damage Rate`) true))
  (set `self.DamageLoopTimerHandle` _returnvalue))

(event `Timer | Stop Damage Loop`
  ;[0 0 0] Damage Overlapping Players
  ;;[0.02431 0.02431 0.02431] Stop Damage Timer
  (`KismetSystemLibrary.K2_ClearAndInvalidateTimerHandle` (`self.DamageLoopTimerHandle`)))

(event `self.LaserCylinder.OnComponentEndOverlap`
  (params (OverlappedComponent :type "PrimitiveComponent Object Reference") (OtherActor :type "Actor Object Reference") (OtherComp :type "PrimitiveComponent Object Reference") (OtherBodyIndex :type Integer))
  ;[0 0 0] Event | Component End Overlap
  ;;[0.02431 0.02431 0.02431] Is it a character?
  (cast `Character` OtherActor)
  ;;[0.02431 0.02431 0.02431] Is Damage Timer Active?
  (if (`KismetSystemLibrary.K2_IsValidTimerHandle` (`self.DamageLoopTimerHandle`))
    ;;[0.02431 0.02431 0.02431] No overlapping Characters left?
    (if (not (> (`KismetArrayLibrary.Array_Length` (`PrimitiveComponent.GetOverlappingActors` (`self.LaserCylinder`) "/Script/Engine.Character")) 0))
      ;;[0.02431 0.02431 0.02431] Stop Timer
      (`self.Timer | Stop Damage Loop`))))

(event `Timer | Damage Loop`
  ;[0 0 0] Damage Overlapping Players
  ;;[0.02431 0.02431 0.02431] Event | Cause Damage
  ;;;[0.07986 0.07986 0.07986] Loop through all players
  (for _array_element (`PrimitiveComponent.GetOverlappingActors` (`self.LaserCylinder`) "/Script/Engine.Character")
    ;;;[0.07986 0.07986 0.07986 1 11] I have a whole system built for Health/Damage that comes with tracking, accounting for world damage vs. player damage, and lots more. Would have done more on this but wanted to keep it short and sweet.
    (`GameplayStatics.ApplyDamage` _array_element (`self.Damage Amount`) null self)))

(fn `DisableLaser`
  (bind _lasercylinder (`self.LaserCylinder`))
  (`PrimitiveComponent.SetCollisionEnabled` _lasercylinder "NoCollision")
  (`SceneComponent.SetVisibility` _lasercylinder false false))

(fn `EnableLaser`
  (bind _lasercylinder (`self.LaserCylinder`))
  (`PrimitiveComponent.SetCollisionEnabled` _lasercylinder "QueryAndPhysics")
  (`SceneComponent.SetVisibility` _lasercylinder true false))

(fn `UserConstructionScript`)