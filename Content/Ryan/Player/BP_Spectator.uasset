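; BP_Spectator is the player's death camera, which shows the death widget and plays a post-process fade and camera move.
; InitializeSpectator caches both camera transforms, waits for the spawn delay, then creates the widget, or destroys the actor if it has no controller (multiplayer is not handled).
; Two timelines, rate-scaled by fade length, drive the post-process vector and, after a further delay, lerp Camera to Camera1's transform with sweep.
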(event `Event | Initialize Spectator`
  (bind _returnvalue (`self.GetController`))
  (bind _returnvalue_2 (/ 1.0 (`self.SpawnFadeLength`)))
  (`self.Initialize Data`)
  ;[1 1 1] Spawn Delay
  (`KismetSystemLibrary.Delay` (`self.Spawn Delay`))
  (`/Engine/EditorBlueprintResources/StandardMacros.IsValid` _returnvalue
    (:`Is Valid`
      (bind _returnvalue_3 (`|CreateWidget` "/Game/Ryan/Player/BP_DeathWidget.BP_DeathWidget_C" (cast `PlayerController` _returnvalue :!pure true)))
      (`/Game/Ryan/Player/BP_DeathWidget.Initialize` _returnvalue_3)
      (`UserWidget.AddToViewport` _returnvalue_3 0)
      ;[1 1 1] Update Play Rate
      (`TimelineComponent.SetPlayRate` (`self.PlayerDeath_CameraFade`) _returnvalue_2)
      (`TimelineComponent.SetPlayRate` (`self.PlayerDeath_CameraMovement`) _returnvalue_2)
      (`|ExecutionSequence`
        (:`then_0`
          ;[1 1 1] Timeline | Camera FX
          (bind (_direction _progress) (`Timeline|PlayerDeath_CameraFade`)
            (:`Update`
              (bind _returnvalue_4 (`KismetMathLibrary.Lerp` 0.0 1.0 _progress))
              (set `CameraComponent.PostProcessSettings` (make `PostProcessSettings` :`ColorGamma` (`KismetMathLibrary.MakeVector4` _returnvalue_4 _returnvalue_4 _returnvalue_4 _returnvalue_4)) (`self.Camera`)) ; If there were other camera settings\nthis would obviously get a bit more complex
            )))
        (:`then_1`
          ;[1 1 1] Camera Movement Delay
          (`KismetSystemLibrary.Delay` (/ _returnvalue_2 (/ 1.0 (`self.Camera_BeginMovement_Percentage`))))
          ;[1 1 1] Timeline | Camera Movement
          (bind (_direction_2 _progress_2) (`Timeline|PlayerDeath_CameraMovement` :!via `PlayFromStart`)
            (:`Update`
              (`SceneComponent.K2_SetWorldTransform` (`self.Camera`) (`KismetMathLibrary.TLerp` (`self.Home_Transform`) (`self.Goal_Transform`) _progress_2) true false))))))
    (:`Is Not Valid`
      (`self.K2_DestroyActor`) ; Multiplayer Implementation would be different here.
    )))

(fn `Initialize Data`
  (set `self.Home_Transform` (`SceneComponent.K2_GetComponentToWorld` (`self.Camera`)))
  (set `self.Goal_Transform` (`SceneComponent.K2_GetComponentToWorld` (`self.Camera1`))))

(fn `UserConstructionScript`)