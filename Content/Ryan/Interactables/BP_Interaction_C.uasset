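; Player interaction component that lets its owner use actors carrying a BP_Interactable_C component.
; On BeginPlay it waits for a valid owner, then caches the owning pawn's first camera via an overridable getter.
; The Interact input line-traces forward from that camera on Visibility, up to InteractionDistance.
; A hit calls Interact inside TraceForInteractable and again in the input event, so each press fires it twice.
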(event `Input | Interact`
  (bind (_valid _return) (`self.TraceForInteractable`))
  (if _valid
    (`/Game/Ryan/Interactables/BP_Interactable_C.Interact` _return (`self.GetOwner`))))

(event `self.ReceiveBeginPlay`
  (bind (_valid _camera) (`self.GetOwningPlayerCamera` 0))
  (`/Game/Ryan/TDT_ML_ActorComponent.WaitForValidity` (`self.GetOwner`) 0.25 30
    (:`IsValid`
      (if _valid
        (set `self.PlayerCameraRef` _camera)))))

(fn `GetOwningPawn`
  (returns (Pawn :type "Pawn Object Reference") (Valid :type Boolean))
  (bind _aspawn (cast `Pawn` (`self.GetOwner`))
    (:`then`
      (return _aspawn true))
    (:`CastFailed`
      (return null false))))

(fn `GetOwningPlayerCamera`
  (params (CameraIndex :type Integer))
  (returns (Valid :type Boolean) (Camera :type "CameraComponent Object Reference"))
  (bind (_pawn _valid) (`self.GetOwningPawn`))
  (bind _output (`|GetArrayItem` (`Actor.K2_GetComponentsByClass` _pawn "/Script/Engine.CameraComponent") CameraIndex))
  ;[0.07986 0.07986 0.07986] Get player camera at index. Can be overriden to change trace logic
  (if _valid
    (`/Engine/EditorBlueprintResources/StandardMacros.IsValid` _output
      (:`Is Valid`
        (return true _output))
      (:`Is Not Valid`
        _)))
  (return false null))

(fn `TraceForInteractable`
  (returns (Valid :type Boolean) (Return :type "/Game/Ryan/Interactables/BP_Interactable_C Object Reference"))
  (bind (_start _end _valid) (`/Game/Ryan/TDT_FL.GetForwardTraceLocations_SceneComponent` (`self.PlayerCameraRef`) (`self.Interaction Distance`)))
  (if _valid
    (bind (_outhit _returnvalue) (`KismetSystemLibrary.LineTraceSingle` _start _end "TraceTypeQuery1"))
    (if _returnvalue
      (bind _returnvalue_2 (`Actor.GetComponentByClass` (`.HitActor` (`GameplayStatics.BreakHitResult` _outhit)) "/Game/Ryan/Interactables/BP_Interactable_C.BP_Interactable_C_C"))
      (`/Engine/EditorBlueprintResources/StandardMacros.IsValid` _returnvalue_2
        (:`Is Valid`
          (`/Game/Ryan/Interactables/BP_Interactable_C.Interact` _returnvalue_2 (`self.GetOwner`))
          (return true _returnvalue_2))
        (:`Is Not Valid`
          _))))
  (return false null))