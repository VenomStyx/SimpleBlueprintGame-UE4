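; Interactable door Blueprint that opens for an interacting actor whose inventory holds the matching key item, consuming one key.
; On BeginPlay it caches the door cube's world location as the start and a GOAL component's location as the target.
; A timeline, rate-scaled by transition length, lerps and teleports the cube between them.
; The transition supports reversing, but only an unconnected test sequence uses it.
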(event `self.ReceiveBeginPlay`
  (`parent.ReceiveBeginPlay`)
  (`self.Init Door Data`))

(event `Event | Begin Door Transition`
  (params (Forward :type Boolean))
  (`TimelineComponent.SetPlayRate` (`self.Timeline | Door Transition`) (/ 1.0 (`self.DoorTransitionLength`)))
  (if Forward
    (bind (_direction _progress) (`Timeline|Timeline | Door Transition` :!label _label)
      (:`Update`
        (`SceneComponent.K2_SetWorldLocation` (`self.Cube`) (`KismetMathLibrary.VLerp` (`self.StartingLocation`) (`self.GoalLocation`) _progress) false true)))
    (else
      (goto _label :!via `Reverse`))))

(event `Request | Open Door`
  (params (`Player Inventory` :type "/Game/Ryan/Items/BP_Inventory_C Object Reference"))
  (bind _keyid (`self.KeyID`))
  ;[0 0 0] Request | Open Door
  ;;[0.02431 0.02431 0.02431] Open door if they have the key
  (if (`.Valid` (`/Game/Ryan/Items/BP_Inventory_C.GetItemByID` `Player Inventory` _keyid))
    (`self.Event | Begin Door Transition` true)
    (`/Game/Ryan/Items/BP_Inventory_C.Request | Remove Item` `Player Inventory` _keyid 1)))

(event `self.Owner Bind | Interaction Initiated`
  (params (`Interacting Actor` :type "Actor Object Reference"))
  ;[0 0 0] Event Owner Bind | Interaction Initiated
  (`self.Request | Open Door` (`/Game/Ryan/TDT_FL.GetInventoryFromActor` `Interacting Actor`)))

(fn `Init Door Data`
  ;[0.07986 0.07986 0.07986] Set Initial Locations
  (set `self.StartingLocation` (`SceneComponent.K2_GetComponentLocation` (`self.Cube`)))
  (set `self.GoalLocation` (`SceneComponent.K2_GetComponentLocation` (`self.GOAL`))))

(fn `UserConstructionScript`)