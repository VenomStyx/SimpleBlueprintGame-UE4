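; BP_HealthAndDamage_C is a component that gives its owning actor health, damage handling and a death notification.
; On BeginPlay it binds to the owner's AnyDamage event and optionally adds a health widget if the owner has a PlayerController.
; Incoming damage is scaled by a multiplier and subtracted from clamped health.
; When health reaches zero, a DoOnce-guarded call fires PlayerKilled with the damage causer.
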(event `self.ReceiveBeginPlay`
  (bind (_return _valid) (`self.GetOwner'sPC`))
  ;[0 0 0] Begin Play
  ;;[0.02431 0.02431 0.02431] Bind Any Damage
  (`self.Bind_OwnerAnyDamage`)
  ;;[0.02431 0.02431 0.02431] Add Health Widget if Setting turned On
  (if (`self.UsesHealthWidget`)
    (if _valid
      (bind _returnvalue (`|CreateWidget` "/Game/Ryan/HealthAndDamage/Widgets/BP_Master_Health_Widget.BP_Master_Health_Widget_C" _return))
      (`UserWidget.AddToViewport` _returnvalue 0))))

(event `Owner Event | Any Damage`
  (params (DamagedActor :type "Actor Object Reference") (Damage :type "Float (double-precision)") (DamageType :type "DamageType Object Reference") (InstigatedBy :type "Controller Object Reference") (DamageCauser :type "Actor Object Reference"))
  ;[0 0 0] Owner Event | Any Damage
  (if (not (`self.IsDead`))
    (`self.ApplyDamage` Damage)
    (`self.IsHealthAtZero`
      (:`true`
        (`/Engine/EditorBlueprintResources/StandardMacros.DoOnce` false
          (:`Completed`
            (`self.Player Killed` DamageCauser)))))))

(fn `AdjustHealth`
  (params (Adjustment :type "Float (double-precision)"))
  (returns (`New Health` :type "Float (double-precision)"))
  (bind _currenthealth (`self.CurrentHealth`))
  (set `self.CurrentHealth` (`KismetMathLibrary.FClamp` (+ _currenthealth Adjustment) 0.0 (`self.MaxHealth`)))
  (return _currenthealth))

(fn `ApplyDamage`
  (params (Damage :type "Float (double-precision)"))
  (returns (`New Health` :type "Float (double-precision)"))
  ;[0.07986 0.07986 0.07986] Calculate Damage & Adjust Health
  (bind _new_health (`self.AdjustHealth` (* (* Damage (`self.DamageMultiplier`)) -1.0)))
  (return _new_health))

(fn `Bind_OwnerAnyDamage`
  (add `Actor.OnTakeAnyDamage` (`self.GetOwner`) (`|CreateDelegate` :!event `Owner Event | Any Damage`)))

(fn `GetOwner'sPC`
  (returns (Return :type "PlayerController Object Reference") (Valid :type Boolean))
  (bind _aspawn (cast `Pawn` (`self.GetOwner`))
    (:`then`
      (bind _asplayer_controller (cast `PlayerController` (`Pawn.GetController` _aspawn))
        (:`then`
          (return _asplayer_controller true))
        (:`CastFailed`
          _)))
    (:`CastFailed`
      _))
  (return null false))

(fn `GetOwnerAsCharacter`
  (returns (Return :type "Character Object Reference") (Valid :type Boolean))
  (bind _ascharacter (cast `Character` (`self.GetOwner`)))
  (return _ascharacter true))

(fn `GetOwnerAsPawn`
  (returns (Return :type "Pawn Object Reference") (Valid :type Boolean))
  (bind _aspawn (cast `Pawn` (`self.GetOwner`))
    (:`then`
      (return _aspawn true))
    (:`CastFailed`
      (return null false))))