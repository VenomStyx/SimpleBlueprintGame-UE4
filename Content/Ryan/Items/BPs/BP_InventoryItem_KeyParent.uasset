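; Parent Blueprint for key inventory items, which applies the item's materials to a two-part key.
; The UpdateItemSettings function creates dynamic material instances for the KeyHandle and ItemMesh components from the first two materials of LocalItem.
; Both instances are stored in the MaterialInstances array.
; The construction script only calls its parent, and the event graph's UpdateItemSettings call is unreachable.
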(fn `UpdateItemSettings`
  ;[0.07986 0.07986 0.07986] Create Material Instance & Add Reference to Array
  ;;[0.3455 0.3455 0.3455] Handle
  (bind _returnvalue (`PrimitiveComponent.CreateDynamicMaterialInstance` (`self.Key_Handle`) 0 (`|GetArrayItem` (`/Game/Ryan/TDT_FL.GetItemMaterials` (`self.LocalItem`))) "None"))
  (`KismetArrayLibrary.Array_Add` (`self.MaterialInstances`) _returnvalue)
  ;;[0.3455 0.3455 0.3455] Key
  (bind _returnvalue_2 (`PrimitiveComponent.CreateDynamicMaterialInstance` (`self.Item_Mesh`) 0 (`|GetArrayItem` (`/Game/Ryan/TDT_FL.GetItemMaterials` (`self.LocalItem`)) 1) "None"))
  (`KismetArrayLibrary.Array_Add` (`self.MaterialInstances`) _returnvalue_2))

(fn `UserConstructionScript`
  (`parent.UserConstructionScript`))