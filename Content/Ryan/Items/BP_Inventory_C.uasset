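; Inventory component that stores item structs in an array, stacking them by item ID.
; Adding raises the count of a matching entry or appends a new one; removing clamps the count and deletes the entry at zero.
; Lookup helpers find items and counts by ID or index.
; Add and remove request events fire the InventoryUpdated dispatcher for widgets, with adding kept as an event to ease future replication.
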(event `AddItemToInventory`
  (params (ItemToAdd :type "/Game/Ryan/Items/Data/BP_InventoryItem_Struct Structure"))
  (bind (_return _item_index) (`self.DoesInventoryContainItem` (`/Game/Ryan/TDT_FL.GetItemID` ItemToAdd)))
  (bind (_return_2 _output) (`self.GetItemAtIndex` _item_index))
  ;[0 0 0] Add Item To Inventory
  ;;[0.02431 0.02431 0.02431] Does Inventory Contain Item?
  (if _return
    ;;[0.02431 0.02431 0.02431] Adjust Item Amount
    (if _return_2
      (`KismetArrayLibrary.Array_Set` (`self.Inventory`) _item_index (`/Game/Ryan/TDT_FL.AdjustItemCount` _output (`/Game/Ryan/TDT_FL.GetItemCount` ItemToAdd)))
      ;;[0.02431 0.02431 0.02431] Event Dispatcher (For Widget)
      (`self.InventoryUpdated` :!label _label))
    (else
      ;;[0.02431 0.02431 0.02431] Simple "Add To Inventory"
      (`KismetArrayLibrary.Array_Add` (`self.Inventory`) ItemToAdd)
      (goto _label))))

(event `Request | Remove Item`
  (params (ID :type Integer) (Amount :type Integer))
  (`self.RemoveItemFromInventory` ID Amount)
  (`self.InventoryUpdated`))

(fn `DoesInventoryContainItem`
  (params (`Item ID` :type Integer))
  (returns (Return :type Boolean) (`Item Index` :type Integer))
  (locals (LocalValidityReturn :type Boolean) (LocalIndexReturn :type Integer))
  ;[0.07986 0.07986 0.07986] Loop through inventory and find Item based on ID
  (for (_array_element _array_index) (`self.Inventory`)
    (if (== (`/Game/Ryan/TDT_FL.GetItemID` _array_element) `Item ID`)
      (set `local.LocalValidityReturn` true)
      (set `local.LocalIndexReturn` _array_index)
      (break)))
  ;[0.3455 0.3455 0.3455] Return
  (return (`local.LocalValidityReturn`) (`local.LocalIndexReturn`)))

(fn `GetInventoryItemCount`
  (returns (`Item Count` :type Integer))
  (return (`KismetArrayLibrary.Array_Length` (`self.Inventory`))))

(fn `GetItemAtIndex`
  (params (`Item Index` :type Integer))
  (returns (Return :type Boolean) (Output :type "/Game/Ryan/Items/Data/BP_InventoryItem_Struct Structure (by ref)"))
  (locals (LocalIndexReturn :type Integer))
  (bind _inventory (`self.Inventory`))
  ;[0.07986 0.07986 0.07986] Return Item at Valid Index
  (if (`KismetArrayLibrary.Array_IsValidIndex` _inventory `Item Index`)
    (return true (`|GetArrayItem` _inventory `Item Index`))
    (else
      (return false))))

(fn `GetItemByID`
  (params (ID :type Integer))
  (returns (Item :type "/Game/Ryan/Items/Data/BP_InventoryItem_Struct Structure") (Valid :type Boolean))
  (bind (_return _item_index) (`self.DoesInventoryContainItem` ID))
  (bind (_return_2 _output) (`self.GetItemAtIndex` _item_index))
  ;[0.07986 0.07986 0.07986] Find Index and Return Item
  (if _return
    (if _return_2
      (return _output true)
      (else
        _)))
  (return (struct) false))

(fn `GetItemCountByID`
  (params (ID :type Integer))
  (returns (`Item Count` :type Integer) (Valid :type Boolean))
  (bind (_item _valid) (`self.GetItemByID` ID))
  ;[0.07986 0.07986 0.07986] Get Item by ID and Return Count
  (if _valid
    (return (`/Game/Ryan/TDT_FL.GetItemCount` _item) true)
    (else
      (return 0 false))))

(fn `RemoveItemFromInventory`
  (params (ID :type Integer) (Amount :type Integer))
  (bind (_return _item_index) (`self.DoesInventoryContainItem` ID))
  (bind (_return_2 _output) (`self.GetItemAtIndex` _item_index))
  (bind (_name _id _blueprintclass _count) (break `/Game/Ryan/Items/Data/BP_InventoryItem_Struct` _output))
  (bind _returnvalue (`KismetMathLibrary.Clamp` (- _count Amount) 0 _count))
  (if _return
    (if _return_2
      (if (<= _returnvalue 0)
        (`KismetArrayLibrary.Array_Remove` (`self.Inventory`) _item_index)
        (else
          (`KismetArrayLibrary.Array_Set` (`self.Inventory`) _item_index (make `/Game/Ryan/Items/Data/BP_InventoryItem_Struct` _name _id _blueprintclass _returnvalue)))))))