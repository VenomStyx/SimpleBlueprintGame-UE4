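; Health and damage component that tracks the owner's current health and announces damage and death.
; On BeginPlay it binds to the owner's AnyDamage event, skipping hits when dead or when the owning BP_FirstPersonCharacter has god mode enabled.
; Damage is scaled by a multiplier and applied as clamped health with a DamageTaken dispatch; reaching zero calls PlayerKilled once with the damage causer.
; The health widget creation here is disconnected, noted as moved to MasterPlayerWidget.
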(event `self.ReceiveBeginPlay`
  ;[0 0 0] Begin Play
  ;;[0.02431 0.02431 0.02431] Bind Any Damage
  (`self.OwnerBind_EventAnyDamage`)
  ;;[0.02431 0.02431 0.02431] Add Health Widget if Setting turned On (Moved but still a viable option)
  (if (`self.UsesHealthWidget`)
    _))

(event `Owner Event | Any Damage`
  (params (DamagedActor :type "Actor Object Reference") (Damage :type "Float (double-precision)") (DamageType :type "DamageType Object Reference") (InstigatedBy :type "Controller Object Reference") (DamageCauser :type "Actor Object Reference"))
  ;[0 0 0] Owner Event | Any Damage
  (if (`self.OwnerCanBeDamaged`)
    (if (not (`self.IsDead`))
      (`self.ApplyDamage` Damage)
      (`self.IsHealthAtZero`
        (:`true`
          (`/Engine/EditorBlueprintResources/StandardMacros.DoOnce` false
            (:`Completed`
              (`self.Player Killed` DamageCauser))))))))

(fn `AdjustHealth`
  (params (Adjustment :type "Float (double-precision)"))
  (returns (`New Health` :type "Float (double-precision)"))
  (bind _currenthealth (`self.CurrentHealth`))
  (set `self.CurrentHealth` (`KismetMathLibrary.FClamp` (+ _currenthealth Adjustment) 0.0 (`self.MaxHealth`)))
  (return _currenthealth))

(fn `ApplyDamage`
  (params (Damage :type "Float (double-precision)"))
  (returns (`New Health` :type "Float (double-precision)"))
  (bind _returnvalue (* (* Damage (`self.DamageMultiplier`)) -1.0))
  ;[0.07986 0.07986 0.07986] Calculate Damage & Adjust Health
  ;;[0.3455 0.3455 0.3455] Any Damage?
  (if (< _returnvalue 0.0)
    (bind _new_health (`self.AdjustHealth` _returnvalue))
    ;[0.07986 0.07986 0.07986] Dispatch
    (`self.DamageTaken`))
  ;[0.07986 0.07986 0.07986] Return
  (return _new_health))

(fn `GetOwner'sPC`
  (returns (Return :type "PlayerController Object Reference") (Valid :type Boolean))
  (bind _aspawn (cast `Pawn` (`self.GetOwner`))
    (:`then`
      (bind _asplayer_controller (cast `PlayerController` (`Pawn.GetController` _aspawn))
        (:`then`
          (return _asplayer_controller true))
        (:`CastFailed`
          _)))
    (:`CastFailed`
      _))
  (return null false))

(fn `OwnerBind_EventAnyDamage`
  (add `Actor.OnTakeAnyDamage` (`self.GetOwner`) (`|CreateDelegate` :!event `Owner Event | Any Damage`)))

(fn `OwnerCanBeDamaged`
  (returns (Return :type Boolean))
  ;[0.07986 0.07986 0.07986] God Mode not Enabled
  (bind _asbp_first_person_character (cast `/Game/TDT_Ryan/Player/BP_FirstPersonCharacter` (`self.GetOwner`)))
  (return (not (`/Game/TDT_Ryan/Player/BP_FirstPersonCharacter.GodModeEnabled` _asbp_first_person_character))))