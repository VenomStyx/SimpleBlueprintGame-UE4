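; Inventory Blueprint that stores item structs in an array, stacking by item ID, with request events for adding and removing items.
; Lookup functions find items and counts by ID through a linear search.
; Adding increases an existing item's count or appends a new entry, while removing clamps the count and deletes entries that reach zero.
; An InventoryUpdated dispatcher notifies the widget of changes, firing after every remove request, even if nothing matched.
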(event `Request | Add Item To Inventory`
  (params (ItemToAdd :type "/Game/TDT_Ryan/Systems/Items/Data/BP_InventoryItem_Struct Structure"))
  ;[0 0 0] Request | Add Item To Inventory
  (`self.AddItemToInventory` ItemToAdd))

(event `Request | Remove Item`
  (params (ID :type Integer) (Amount :type Integer))
  ;[0 0 0] Request | Remove Item
  (`self.RemoveItemFromInventory` ID Amount)
  (`self.InventoryUpdated`))

(fn `AddItemToInventory`
  (params (InputPin :type "/Game/TDT_Ryan/Systems/Items/Data/BP_InventoryItem_Struct Structure"))
  (bind (_return _item_index) (`self.DoesInventoryContainItem` (`/Game/TDT_Ryan/Game/Utilities/TDT_FL.GetItemID` InputPin)))
  (bind (_return_2 _output) (`self.GetItemAtIndex` _item_index))
  ;[0.02431 0.02431 0.02431] Does Inventory Contain Item?
  (if _return
    ;[0.02431 0.02431 0.02431] Adjust Item Amount
    (if _return_2
      (`KismetArrayLibrary.Array_Set` (`self.Inventory`) _item_index (`/Game/TDT_Ryan/Game/Utilities/TDT_FL.AdjustItemCount` _output (`/Game/TDT_Ryan/Game/Utilities/TDT_FL.GetItemCount` InputPin)))
      ;[0.02431 0.02431 0.02431] Event Dispatcher (For Widget)
      (`self.InventoryUpdated` :!label _label))
    (else
      ;[0.02431 0.02431 0.02431] Simple "Add To Inventory"
      (`KismetArrayLibrary.Array_Add` (`self.Inventory`) InputPin)
      (goto _label))))

(fn `DoesInventoryContainItem`
  (params (`Item ID` :type Integer))
  (returns (Return :type Boolean) (`Item Index` :type Integer))
  (locals (LocalValidityReturn :type Boolean) (LocalIndexReturn :type Integer))
  ;[0.07986 0.07986 0.07986] Loop through inventory and find Item based on ID
  (for (_array_element _array_index) (`self.Inventory`)
    (if (== (`/Game/TDT_Ryan/Game/Utilities/TDT_FL.GetItemID` _array_element) `Item ID`)
      (set `local.LocalValidityReturn` true)
      (set `local.LocalIndexReturn` _array_index)
      (break)))
  ;[0.3455 0.3455 0.3455] Return
  (return (`local.LocalValidityReturn`) (`local.LocalIndexReturn`)))

(fn `GetInventoryItemCount`
  (returns (`Item Count` :type Integer))
  (return (`KismetArrayLibrary.Array_Length` (`self.Inventory`))))

(fn `GetItemAtIndex`
  (params (`Item Index` :type Integer))
  (returns (Return :type Boolean) (Output :type "/Game/TDT_Ryan/Systems/Items/Data/BP_InventoryItem_Struct Structure (by ref)"))
  (locals (LocalIndexReturn :type Integer))
  (bind _inventory (`self.Inventory`))
  ;[0.07986 0.07986 0.07986] Return Item at Valid Index
  (if (`KismetArrayLibrary.Array_IsValidIndex` _inventory `Item Index`)
    (return true (`|GetArrayItem` _inventory `Item Index`))
    (else
      (return false))))

(fn `GetItemByID`
  (params (ID :type Integer))
  (returns (Item :type "/Game/TDT_Ryan/Systems/Items/Data/BP_InventoryItem_Struct Structure") (Valid :type Boolean))
  (bind (_return _item_index) (`self.DoesInventoryContainItem` ID))
  (bind (_return_2 _output) (`self.GetItemAtIndex` _item_index))
  ;[0.07986 0.07986 0.07986] Find Index and Return Item
  (if _return
    (if _return_2
      (return _output true)
      (else
        _)))
  (return (struct) false))

(fn `GetItemCountByID`
  (params (ID :type Integer))
  (returns (`Item Count` :type Integer) (Valid :type Boolean))
  (bind (_item _valid) (`self.GetItemByID` ID))
  ;[0.07986 0.07986 0.07986] Get Item by ID and Return Count
  (if _valid
    (return (`/Game/TDT_Ryan/Game/Utilities/TDT_FL.GetItemCount` _item) true)
    (else
      (return 0 false))))

(fn `RemoveItemFromInventory`
  (params (ID :type Integer) (Amount :type Integer))
  (locals (LocalTempIndex :type Integer :default 0))
  (bind (_return _item_index) (`self.DoesInventoryContainItem` ID))
  (bind (_return_2 _output) (`self.GetItemAtIndex` (`local.LocalTempIndex`)))
  (bind (_name _id _blueprintclass _count) (break `/Game/TDT_Ryan/Systems/Items/Data/BP_InventoryItem_Struct` _output))
  (bind _returnvalue (`KismetMathLibrary.Clamp` (- _count Amount) 0 _count))
  ;[0.07986 0.07986 0.07986] Find Inventory Item Index
  (if _return
    (set `local.LocalTempIndex` _item_index)
    ;[0.07986 0.07986 0.07986] Get Item Data
    (if _return_2
      ;[0.07986 0.07986 0.07986] Adjust Amount, Check if item count is 0
      (if (<= _returnvalue 0)
        ;[0.07986 0.07986 0.07986] Remove or Adjust
        (`KismetArrayLibrary.Array_Remove` (`self.Inventory`) (`local.LocalTempIndex`))
        (else
          (`KismetArrayLibrary.Array_Set` (`self.Inventory`) (`local.LocalTempIndex`) (make `/Game/TDT_Ryan/Systems/Items/Data/BP_InventoryItem_Struct` _name _id _blueprintclass _returnvalue)))))))