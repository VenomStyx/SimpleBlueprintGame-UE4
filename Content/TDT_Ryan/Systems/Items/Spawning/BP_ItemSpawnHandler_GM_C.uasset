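; Item spawn handler that, on BeginPlay, populates the level with items from a list of ID and amount requirements.
; It first groups all BP_ItemSpawn actors by item ID for cheaper lookup.
; Each requirement spawns its item class at random matching spawners, removing used points from the pool.
; Requirements are processed recursively, with a list-length check against infinite loops, and completion is broadcast once none remain.
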(event `self.ReceiveBeginPlay`
  ;[0 0 0] Event | Begin Play
  (`self.Initialize Item Spawning`))

(event `Initialize Item Spawning`
  ;[0 0 0] Event | Initialize Item Spawning
  ;;[0.02431 0.02431 0.02431] Update Spawn Requirements
  (set `self.LocalItemSpawnRequirements` (`self.ItemSpawnRequirements`))
  ;;[0.02431 0.02431 0.02431] Sort Item Spawners
  (`self.GenerateSortedItemSpawners`)
  ;;[0.02431 0.02431 0.02431] Initiate Spawning
  (`self.Spawn Item Requirements`))

(event `Spawn Item Requirements`
  ;[0 0 0] Event | Spawn Item Requirements
  (if (`self.AnySpawnRequirementsLeft`)
    (`self.SpawnItem` (`|GetArrayItem` (`self.LocalItemSpawnRequirements`))) ; Spawn until no requirements left
    (else
      (`self.ItemSpawnComplete`))))

(fn `AnySpawnRequirementsLeft`
  (returns (ReturnValue :type Boolean))
  (return (> (`KismetArrayLibrary.Array_Length` (`self.LocalItemSpawnRequirements`)) 0)))

(fn `GenerateSortedItemSpawners`
  (locals (LocalIDsToSpawn :type "Array of Integer"))
  (bind _localidstospawn (`local.LocalIDsToSpawn`))
  ;[0.07986 0.07986 0.07986] Create list of Sorted Spawners
  ;;[0.3455 0.3455 0.3455] Get Required IDs
  (for _array_element (`self.ItemSpawnRequirements`)
    (bind _itemid (break `/Game/TDT_Ryan/Systems/Items/Data/BP_ItemSpawnRequirements_Struct` _array_element))
    (if (not (`KismetArrayLibrary.Array_Contains` _localidstospawn _itemid))
      (`KismetArrayLibrary.Array_Add` _localidstospawn _itemid)))
  (bind _outactors (`GameplayStatics.GetAllActorsOfClass` "/Game/TDT_Ryan/Systems/Items/Spawning/BP_ItemSpawn.BP_ItemSpawn_C"))
  ;;[0.3455 0.3455 0.3455] Loop & Sort Spawners by ID
  (for _array_element_2 _outactors
    (bind _itemid_2 (`/Game/TDT_Ryan/Systems/Items/Spawning/BP_ItemSpawn.ItemID` _array_element_2))
    (bind (_spawnerindex _found) (`self.GetItemSpawnerIndexByID` _itemid_2))
    (if _found
      ;;[0.3455 0.3455 0.3455] Add to Existing Entry
      (`KismetArrayLibrary.Array_Add` (`.AvailableSpawns_6_BEEA93C54DEAF8FA9FB566825878CE25` (break `/Game/TDT_Ryan/Systems/Items/Data/BP_ItemSpawner_Struct` (`|GetArrayItem` (`self.SortedItemSpawners`) _spawnerindex))) _array_element_2)
      (else
        ;;[0.3455 0.3455 0.3455] Create new entry
        (`KismetArrayLibrary.Array_Add` (`self.SortedItemSpawners`) (make `/Game/TDT_Ryan/Systems/Items/Data/BP_ItemSpawner_Struct` _itemid_2 (`|MakeArray` _array_element_2)))))))

(fn `GetItemSpawnerIndexByID`
  (params (ID :type Integer))
  (returns (SpawnerIndex :type Integer) (Found :type Boolean))
  (locals (LocalFound :type Boolean) (LocalIndex :type Integer))
  ;[0.07986 0.07986 0.07986] Loop and find index of Item ID
  (for (_array_element _array_index) (`self.SortedItemSpawners`)
    (if (== (`.ItemID_5_21679F6848F53696E7B6EB930F55BAF9` (break `/Game/TDT_Ryan/Systems/Items/Data/BP_ItemSpawner_Struct` _array_element)) ID)
      (set `local.LocalFound` true)
      (set `local.LocalIndex` _array_index)
      (break)))
  ;[0.07986 0.07986 0.07986] Return
  (return (`local.LocalIndex`) (`local.LocalFound`)))

(fn `GetRandomSpawnerByID`
  (params (ID :type Integer))
  (returns (Valid :type Boolean) (Spawn :type "/Game/TDT_Ryan/Systems/Items/Spawning/BP_ItemSpawn Object Reference"))
  (bind (_valid _available_spawns) (`self.GetSpawnersByID` ID))
  (bind _output (`|GetArrayItem` _available_spawns (`KismetMathLibrary.RandomIntegerInRange` 0 (`KismetArrayLibrary.Array_LastIndex` _available_spawns))))
  ;[0.07986 0.07986 0.07986] Get Random Sorted Spawner by ID
  (if _valid
    (`/Engine/EditorBlueprintResources/StandardMacros.IsValid` _output
      (:`Is Valid`
        (return true _output))
      (:`Is Not Valid`
        _)))
  (return false null))

(fn `GetSpawnersByID`
  (params (ID :type Integer))
  (returns (Valid :type Boolean) (`Available Spawns` :type "Array of /Game/TDT_Ryan/Systems/Items/Spawning/BP_ItemSpawn Object Reference"))
  (bind (_spawnerindex _found) (`self.GetItemSpawnerIndexByID` ID))
  ;[0.07986 0.07986 0.07986] Find Spawners by ID in Sorted Item Struct
  (if _found
    (return true (`.AvailableSpawns_6_BEEA93C54DEAF8FA9FB566825878CE25` (break `/Game/TDT_Ryan/Systems/Items/Data/BP_ItemSpawner_Struct` (`|GetArrayItem` (`self.SortedItemSpawners`) _spawnerindex))))
    (else
      (return false))))

(fn `RemoveLocalItemRequirement`
  (params (Item :type "/Game/TDT_Ryan/Systems/Items/Data/BP_ItemSpawnRequirements_Struct Structure (by ref)"))
  (`KismetArrayLibrary.Array_RemoveItem` (`self.LocalItemSpawnRequirements`) Item))

(fn `RemoveSpawnerFromReferences`
  (params (`Spawner To Remove` :type "/Game/TDT_Ryan/Systems/Items/Spawning/BP_ItemSpawn Object Reference"))
  (returns (Success :type Boolean))
  (bind (_spawnerindex _found) (`self.GetItemSpawnerIndexByID` (`/Game/TDT_Ryan/Systems/Items/Spawning/BP_ItemSpawn.ItemID` `Spawner To Remove`)))
  ;[0.07986 0.07986 0.07986] Remove Spawner from SortedSpawners Variable
  (`/Engine/EditorBlueprintResources/StandardMacros.IsValid` `Spawner To Remove`
    (:`Is Valid`
      (if _found
        (bind _returnvalue (`KismetArrayLibrary.Array_RemoveItem` (`.AvailableSpawns_6_BEEA93C54DEAF8FA9FB566825878CE25` (break `/Game/TDT_Ryan/Systems/Items/Data/BP_ItemSpawner_Struct` (`|GetArrayItem` (`self.SortedItemSpawners`) _spawnerindex))) `Spawner To Remove`))
        (return _returnvalue)
        (else
          _)))
    (:`Is Not Valid`
      _))
  (return false))

(fn `SpawnItem`
  (params (Item :type "/Game/TDT_Ryan/Systems/Items/Data/BP_ItemSpawnRequirements_Struct Structure"))
  (locals (`Local Chosen Spawn` :type "/Game/TDT_Ryan/Systems/Items/Spawning/BP_ItemSpawn Object Reference") (LocalItemRequirementData :type "/Game/TDT_Ryan/Systems/Items/Data/BP_ItemSpawnRequirements_Struct Structure") (BegginingSpawnRequirementsLength :type Integer :default 0))
  (bind (_itemid _amounttospawn) (break `/Game/TDT_Ryan/Systems/Items/Data/BP_ItemSpawnRequirements_Struct` (`local.LocalItemRequirementData`)))
  (bind (_valid _item_data) (`/Game/TDT_Ryan/Game/Utilities/TDT_FL.GetItemDataByID` _itemid))
  (bind (_valid_2 _spawn) (`self.GetRandomSpawnerByID` _itemid))
  ;[0.07986 0.07986 0.07986] Init Local Data
  (set `local.BegginingSpawnRequirementsLength` (`KismetArrayLibrary.Array_Length` (`self.LocalItemSpawnRequirements`)))
  (set `local.LocalItemRequirementData` Item)
  ;[0.07986 0.07986 0.07986] Get Item Data and Amount to Spawn
  (if _valid
    ;[0.07986 0.07986 0.07986] Spawn Loop | Find Random Spawn, Spawn Actor, Remove Spawner from References.
    (for _ (range 1 (+ _amounttospawn 1))
      (`/Engine/EditorBlueprintResources/StandardMacros.IsValid` _spawn ; Remove Requirement if no spawns left
        (:`Is Valid`
          (set `local.Local Chosen Spawn` _spawn)
          (if _valid_2
            (bind _returnvalue (`|SpawnActorFromClass` (`/Game/TDT_Ryan/Game/Utilities/TDT_FL.GetItemClass` _item_data) (`Actor.GetTransform` (`local.Local Chosen Spawn`)) "Undefined" "OverrideRootScale" null null))
            (`/Engine/EditorBlueprintResources/StandardMacros.IsValid` _returnvalue
              (:`Is Valid`
                (`self.RemoveSpawnerFromReferences` (`local.Local Chosen Spawn`))))))))
    ;[0.07986 0.07986 0.07986] Remove Local Spawn Requirement, Ensure no Infinite Loop, Spawn next Item
    (`self.RemoveLocalItemRequirement` (`local.LocalItemRequirementData`))
    (if (!= (`local.BegginingSpawnRequirementsLength`) (`KismetArrayLibrary.Array_Length` (`self.LocalItemSpawnRequirements`)))
      (`self.Spawn Item Requirements`))))