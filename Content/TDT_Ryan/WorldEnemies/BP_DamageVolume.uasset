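; BP_DamageVolume is a world hazard box that damages every Character inside it once per second.
; The first Character to enter starts a looping timer, with an immediate first hit, and each tick applies DamagePerSecond through ApplyDamage to all overlapping Characters.
; The timer is cleared when the last Character leaves, so it only runs while occupied.
; The construction script sizes the box from its extent variables.
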(event `StartDamageTimer`
  ;[0 0 0] Damage Overlapping Players
  ;;[0.02431 0.02431 0.02431] Start Damage Timer
  (`self.Event_CauseDamage`)
  (bind _returnvalue (`KismetSystemLibrary.K2_SetTimerDelegate` (delegate `Event_CauseDamage`) 1.0 true))
  (set `self.DamageTimer` _returnvalue))

(event `StopDamageTimer`
  ;[0 0 0] Damage Overlapping Players
  ;;[0.02431 0.02431 0.02431] Stop Damage Timer
  (`KismetSystemLibrary.K2_ClearAndInvalidateTimerHandle` (`self.DamageTimer`)))

(event `self.Box.OnComponentBeginOverlap`
  (params (OverlappedComponent :type "PrimitiveComponent Object Reference") (OtherActor :type "Actor Object Reference") (OtherComp :type "PrimitiveComponent Object Reference") (OtherBodyIndex :type Integer) (bFromSweep :type Boolean) (SweepResult :type "HitResult Structure (by ref)"))
  ;[0 0 0] Event | Component Begin Overlap
  ;;[0.02431 0.02431 0.02431] Is it a character?
  (cast `Character` OtherActor)
  ;;[0.02431 0.02431 0.02431] If damage timer isn't already started, begin damage timer
  (if (not (`KismetSystemLibrary.K2_IsValidTimerHandle` (`self.DamageTimer`)))
    (`self.StartDamageTimer`)))

(event `Event_CauseDamage`
  ;[0 0 0] Damage Overlapping Players
  ;;[0.02431 0.02431 0.02431] Event | Cause Damage
  ;;;[0.07986 0.07986 0.07986] Loop through all players
  (for _array_element (`PrimitiveComponent.GetOverlappingActors` (`self.Box`) "/Script/Engine.Character")
    ;;;[0.07986 0.07986 0.07986 1 11] I have a whole system built for Health/Damage that comes with tracking, accounting for world damage vs. player damage, and lots more. Would have done more on this but wanted to keep it short and sweet.
    (`GameplayStatics.ApplyDamage` _array_element (`self.Damage Per Second`) null self)))

(event `self.Box.OnComponentEndOverlap`
  (params (OverlappedComponent :type "PrimitiveComponent Object Reference") (OtherActor :type "Actor Object Reference") (OtherComp :type "PrimitiveComponent Object Reference") (OtherBodyIndex :type Integer))
  ;[0 0 0] Event | Component End Overlap
  ;;[0.02431 0.02431 0.02431] Is it a character?
  (cast `Character` OtherActor)
  ;;[0.02431 0.02431 0.02431] Is Damage Timer Active?
  (if (`KismetSystemLibrary.K2_IsValidTimerHandle` (`self.DamageTimer`))
    ;;[0.02431 0.02431 0.02431] No overlapping Characters left?
    (if (not (> (`KismetArrayLibrary.Array_Length` (`PrimitiveComponent.GetOverlappingActors` (`self.Box`) "/Script/Engine.Character")) 0))
      ;;[0.02431 0.02431 0.02431] Stop Timer
      (`self.StopDamageTimer`))))

(fn `UserConstructionScript`
  (`BoxComponent.SetBoxExtent` (`self.Box`) (`KismetMathLibrary.MakeVector` (`self.Box Extent (X)`) (`self.Box Extent (Y)`) (`self.Box Extent (Z)`)) true))