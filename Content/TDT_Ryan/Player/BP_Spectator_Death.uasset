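; Death spectator that, once initialized with a valid controller, shows the death screen and plays a camera sequence.
; It caches the transforms of two camera components, waits a spawn delay, then adds BP_DeathWidget with a visible cursor and Game and UI input.
; Two timelines rate-scaled by fade length drive the sequence: a post-process fade, then a delayed, swept camera move toward the second camera's transform.
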(event `Event | Initialize Spectator`
  ;[0 0 0] Event | Initialize Spectator
  (`/Engine/EditorBlueprintResources/StandardMacros.IsValid` (`self.GetController`) ; Make sure controller is valid before\nproceeding
    (:`Is Valid`
      ;;[0.02431 0.02431 0.02431] Initialize Data
      (`self.Initialize Data`)
      ;;[0.02431 0.02431 0.02431] Spawn Delay
      (`KismetSystemLibrary.Delay` (`self.Spawn Delay`))
      ;;[0.02431 0.02431 0.02431] Widget
      (`self.Initialize Death Widget`)
      ;;[0.02431 0.02431 0.02431] Play Animation
      (`self.Event | Play Camera Animation`))))

(event `Event | Play Camera Animation`
  (bind _returnvalue (/ 1.0 (`self.SpawnFadeLength`)))
  ;[0 0 0] Event | Play Camera Animation
  ;;[0.02431 0.02431 0.02431] Update Play Rate
  (`TimelineComponent.SetPlayRate` (`self.PlayerDeath_CameraFade`) _returnvalue)
  (`TimelineComponent.SetPlayRate` (`self.PlayerDeath_CameraMovement`) _returnvalue)
  ;;[0.02431 0.02431 0.02431] Begin Camera Fade
  (`self.Event | Begin Camera FX Fade`)
  ;;[0.02431 0.02431 0.02431] Delay
  (`KismetSystemLibrary.Delay` (/ _returnvalue (/ 1.0 (`self.Camera_BeginMovement_Percentage`))))
  ;;[0.02431 0.02431 0.02431] Begin Camera Movement
  (`self.Event | Begin Camera Movement`))

(event `Event | Begin Camera FX Fade`
  ;[0 0 0] Event | Begin Camera FX Fade
  ;;[0.02431 0.02431 0.02431] Timeline | Camera FX
  (bind (_direction _progress) (`Timeline|PlayerDeath_CameraFade` :!via `PlayFromStart`)
    (:`Update`
      (bind _returnvalue (`KismetMathLibrary.Lerp` 0.0 1.0 _progress))
      (set `CameraComponent.PostProcessSettings` (make `PostProcessSettings` :`ColorGamma` (`KismetMathLibrary.MakeVector4` _returnvalue _returnvalue _returnvalue _returnvalue)) (`self.Camera`)) ; If there were other camera settings\nthis would obviously get a bit more complex
    )))

(event `Event | Begin Camera Movement`
  ;[0 0 0] Event | Begin Camera Movement
  ;;[0.02431 0.02431 0.02431] Timeline | Camera Movement
  (bind (_direction _progress) (`Timeline|PlayerDeath_CameraMovement` :!via `PlayFromStart`)
    (:`Update`
      (`SceneComponent.K2_SetWorldTransform` (`self.Camera`) (`KismetMathLibrary.TLerp` (`self.Home_Transform`) (`self.Goal_Transform`) _progress) true false))))

(fn `Initialize Data`
  ;[0.07986 0.07986 0.07986] Camera
  (set `self.Home_Transform` (`SceneComponent.K2_GetComponentToWorld` (`self.Camera`)))
  (set `self.Goal_Transform` (`SceneComponent.K2_GetComponentToWorld` (`self.Camera1`))))

(fn `Initialize Death Widget`
  ;[0.07986 0.07986 0.07986] Create, Initialize, and Add to Viewport
  (bind _returnvalue (`|CreateWidget` "/Game/TDT_Ryan/Player/Widgets/BP_DeathWidget.BP_DeathWidget_C" (cast `PlayerController` (`self.GetController`) :!pure true)))
  (`UserWidget.AddToViewport` _returnvalue 0)
  ;[0.07986 0.07986 0.07986] Show Cursor and Update Input
  (bind _asplayer_controller (cast `PlayerController` (`self.GetController`)))
  (set `PlayerController.bShowMouseCursor` true _asplayer_controller)
  (`WidgetBlueprintLibrary.SetInputMode_GameAndUIEx` _asplayer_controller _returnvalue "LockAlways" false))

(fn `UserConstructionScript`)